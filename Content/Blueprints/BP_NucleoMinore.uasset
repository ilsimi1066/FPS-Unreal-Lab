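; BP_NucleoMinore is a destructible minor core actor that shows its remaining health through its sphere's color.
; On BeginPlay it creates a dynamic instance of M_Nucleo and applies it to NucleoSphere.
; AnyDamage reduces Health, lerps the Color parameter by health ratio from red at full toward white at zero, then destroys the actor once health runs out.
; Debug strings print along the way.
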(event EventBeginPlay
  (bind _returnvalue (Rendering|Material|CreateDynamicMaterialInstance (Variables|Default|GetNucleoSphere) 0 "/Game/material/M_Nucleo.M_Nucleo" "None" :!class /Script/Engine.PrimitiveComponent))
  (Development|PrintString "Sono Colorato" true true "(R=1.000000,G=0.357252,B=0.893060,A=1.000000)")
  (Variables|Default|SetDynamicMaterial _returnvalue)
  (Rendering|Material|SetMaterial (Variables|Default|GetNucleoSphere) 0 (Variables|Default|GetDynamicMaterial)))

(event Collision|EventActorBeginOverlap
  (params (OtherActor :type Actor%20Object%20Reference)))

(event EventTick
  (params (DeltaSeconds :type Float%20%28single-precision%29)))

(event Game|Damage|EventAnyDamage
  (params (Damage :type Float%20%28single-precision%29) (DamageType :type Damage%20Type%20Object%20Reference) (InstigatedBy :type Controller%20Object%20Reference) (DamageCauser :type Actor%20Object%20Reference))
  (bind _output_get (Variables|Default|SetHealth (- (Variables|Default|GetHealth) Damage)))
  (Utilities|FlowControl|Sequence
    (:then_0
      (Development|PrintString (Utilities|String|ToString(Float) (Variables|Default|GetHealth)) true true "(R=0.234781,G=1.000000,B=0.154555,A=1.000000)")
      (Rendering|Material|SetVectorParameterValue (Variables|Default|GetDynamicMaterial) "Color" (Math|Color|Lerp(LinearColor) "(R=1.000000,G=1.000000,B=1.000000,A=1.000000)" "(R=1.000000,G=0.000000,B=0.000000,A=1.000000)" (/ (Variables|Default|GetHealth) (Variables|Default|GetMaxHealth))) :!class /Script/Engine.MaterialInstanceDynamic)
      (Development|PrintString "DOP F" true true "(R=1.000000,G=0.000584,B=0.007133,A=1.000000)"))
    (:then_1
      (if (<= _output_get 0.0)
        (Development|PrintString "Nucleo Distrutto" true true "(R=1.000000,G=0.005553,B=0.000000,A=1.000000)")
        (Actor|DestroyActor)))))

(fn ConstructionScript)