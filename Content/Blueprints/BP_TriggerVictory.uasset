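; BP_TriggerVictory is a trigger actor that ends the game in victory when the player's first-person character overlaps it.
; On overlap it fades out the character's normal and fury audio components and shows the UI_Vittoria widget.
; It then pauses the game, plays the victory sound in 2D and shows the mouse cursor.
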(event Collision|EventActorBeginOverlap
  (params (OtherActor :type Actor%20Object%20Reference))
  (bind _asbp_first_person_character (Utilities|Casting|CastToBP_FirstPersonCharacter OtherActor))
  (Audio|Components|Audio|FadeOut (Variables|/Game/Blueprints/FirstPerson/BP_FirstPersonCharacter.BP_FirstPersonCharacter_C|GetAudio_normal _asbp_first_person_character) 1.5 0.0 "Linear" :!class /Script/Engine.AudioComponent)
  (bind _returnvalue (UserInterface|CreateWidget "/Game/Blueprints/UI_Vittoria.UI_Vittoria_C"))
  (UserInterface|Viewport|AddtoViewport _returnvalue 0)
  (Game|SetGamePaused true)
  (Audio|SpawnSound2D (Variables|Default|GetAudio%20vittoria) 1.0 1.0 0.0 0)
  (Variables|/Script/Engine.PlayerController|SetbShowMouseCursor (Game|GetPlayerController 0) true))

(fn ConstructionScript)