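; BP_NucleoMaggiore is a destructible core whose sphere travels along a spline, optionally looping, and opens its linked door when destroyed.
; The first hit activates timed spawning of BP_enemyNucleo AI at SpawnPoints flagged unoccupied.
; Later hits tint the dynamic material from white toward red and check for death.
; Random point selection repeats per use, so checked, spawned and marked points can differ.
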(event Custom|SpawnEnemy
  (bind _spawnpoints (Variables|Default|GetSpawnPoints))
  (bind _spawnpoints_2 (Variables|Default|GetSpawnPoints))
  (bind _returnvalue (Utilities|Array|Length _spawnpoints))
  (bind _returnvalue_2 (- _returnvalue 1))
  (bind _returnvalue_3 (Math|Random|RandomIntegerinRange 0 _returnvalue_2))
  (bind _output (Utilities|Array|Get(acopy) _spawnpoints_2 _returnvalue_3))
  (if (not (Variables|/Game/Blueprints/BP_Enemy_SpawnPoint.BP_Enemy_SpawnPoint_C|GetIsOccupied _output))
    (bind _returnvalue_4 (AI|SpawnAIFromClass "/Game/Blueprints/TP/BP_enemyNucleo.BP_enemyNucleo_C" "/Game/Blueprints/TP/BT_EnemyBase.BT_EnemyBase" (Transformation|GetActorLocation _output) "0, 0, 0" false 0))
    (bind _asbp_enemy_nucleo (Utilities|Casting|CastToBP_enemyNucleo _returnvalue_4))
    (Variables|/Game/Blueprints/TP/BP_enemyNucleo.BP_enemyNucleo_C|SetMySpawnPoint _asbp_enemy_nucleo _output)
    (Variables|/Game/Blueprints/BP_Enemy_SpawnPoint.BP_Enemy_SpawnPoint_C|SetIsOccupied _output true)))

(event EventBeginPlay
  (Rendering|Material|CreateDynamicMaterialInstance (Variables|Default|GetNucleoSphere) 0 "/Game/material/M_Nucleo.M_Nucleo" "None" :!class /Script/Engine.PrimitiveComponent)
  (Development|PrintString "Sono Colorato" true true "(R=1.000000,G=0.357252,B=0.893060,A=1.000000)"))

(event Game|Damage|EventAnyDamage
  (params (Damage :type Float%20%28single-precision%29) (DamageType :type Damage%20Type%20Object%20Reference) (InstigatedBy :type Controller%20Object%20Reference) (DamageCauser :type Actor%20Object%20Reference))
  (bind _output_get (Variables|Default|SetHealth (- (Variables|Default|GetHealth) Damage)))
  (if (Variables|Default|GetIsDamaged)
    (Utilities|FlowControl|Sequence
      (:then_0
        (Development|PrintString (Utilities|String|ToString(Float) (Variables|Default|GetHealth)) true true "(R=0.234781,G=1.000000,B=0.154555,A=1.000000)")
        (Rendering|Material|SetVectorParameterValueonMaterials (Variables|Default|GetNucleoSphere) "NucleoColor" (Math|Conversions|ToVector(LinearColor) (Math|Color|Lerp(LinearColor) (Math|Color|MakeColor 1.0 1.0 1.0) (Math|Color|MakeColor 1.0 (- 1.0 (- 1.0 (Math|Float|NormalizetoRange (Variables|Default|GetHealth) 0.0 (Variables|Default|GetMaxHealth)))) (- 1.0 (- 1.0 (Math|Float|NormalizetoRange (Variables|Default|GetHealth) 0.0 (Variables|Default|GetMaxHealth))))) 1.0)))
        (Development|PrintString "DOP F" true true "(R=1.000000,G=0.000584,B=0.007133,A=1.000000)")
        (Development|PrintString (Utilities|String|ToString(Float) (- 1.0 (Math|Float|NormalizetoRange (Variables|Default|GetHealth) 0.0 (Variables|Default|GetMaxHealth)))) true true "(R=0.932928,G=1.000000,B=0.231307,A=1.000000)"))
      (:then_1
        (if (<= _output_get 0.0)
          (Development|PrintString "Nucleo Distrutto" true true "(R=1.000000,G=0.401322,B=0.000000,A=1.000000)")
          (Default|OpenDoor (Variables|Door|GetLinkedDoor))
          (Actor|DestroyActor))))
    (else
      (Variables|Default|SetIsDamaged true)
      (Variables|Default|SetCurrentSpawnTimer (Variables|EnemySpawn|GetSpawnTimerDuration))
      (Development|PrintString "Spawn!" true true "(R=1.000000,G=0.401322,B=0.000000,A=1.000000)"))))

(event EventTick
  (params (DeltaSeconds :type Float%20%28single-precision%29))
  (Utilities|FlowControl|Sequence
    (:then_0
      (bind _output_get (Variables|Default|SetPositionOnSpline (+ (* DeltaSeconds (Variables|Default|GetSpeedOnSpline)) (Variables|Default|GetPositionOnSpline))))
      (Transformation|SetWorldTransform (Variables|Default|GetNucleoSphere) (Spline|GetTransformatDistanceAlongSpline (Variables|Default|GetSpline) _output_get "World" false) false false)
      (if (Variables|Default|GetLoop)
        (if (>= (Variables|Default|GetPositionOnSpline) (Spline|GetSplineLength (Variables|Default|GetSpline)))
          (Variables|Default|SetPositionOnSpline 0.0))))
    (:then_1
      (if (Variables|Default|GetIsDamaged)
        (Variables|Default|SetCurrentSpawnTimer (- (Variables|Default|GetCurrentSpawnTimer) DeltaSeconds))
        (if (<= (Variables|Default|GetCurrentSpawnTimer) 0.0)
          (CallFunction|SpawnEnemy)
          (Variables|Default|SetCurrentSpawnTimer (Variables|EnemySpawn|GetSpawnTimerDuration)))))))

(fn ConstructionScript)