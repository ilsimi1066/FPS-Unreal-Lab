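; BP_MovingNucleo is an actor that moves its NucleoSphere component along a spline path.
; Each Tick advances a distance by SpeedOnSpline times delta time and sets the sphere's world transform from the spline at that distance, ignoring spline scale and without sweeping.
; When Loop is enabled, the distance resets to zero once it reaches the spline length.
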(event EventTick
  (params (DeltaSeconds :type Float%20%28single-precision%29))
  (bind _output_get (Variables|Default|SetPositionOnSpline (+ (* DeltaSeconds (Variables|Default|GetSpeedOnSpline)) (Variables|Default|GetPositionOnSpline))))
  (Transformation|SetWorldTransform (Variables|Default|GetNucleo%20Sphere) (Spline|GetTransformatDistanceAlongSpline (Variables|Default|GetSpline) _output_get "World" false) false false)
  (if (Variables|Default|GetLoop)
    (if (>= (Variables|Default|GetPositionOnSpline) (Spline|GetSplineLength (Variables|Default|GetSpline)))
      (Variables|Default|SetPositionOnSpline 0.0))))

(fn ConstructionScript)