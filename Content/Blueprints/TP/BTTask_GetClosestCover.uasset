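; Behavior tree task that finds the nearest cover for a BP_enemyBase pawn and writes it to the blackboard.
; It sphere-overlaps WorldDynamic objects within RadiusCheck, keeps the closest actor tagged "Cover" and stores it in the BBCover key.
; It fails only if the pawn cast fails, succeeding even when no cover is found, and TargetCover is not cleared before the search.
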(event EventReceiveExecuteAI
  (params (OwnerController :type AI%20Controller%20Object%20Reference) (ControlledPawn :type Pawn%20Object%20Reference))
  (bind _asbp_enemy_base (Utilities|Casting|CastToBP_enemyBase ControlledPawn)
    (:then
      (Variables|Default|SetMinDistance (+ (Variables|Default|GetRadiusCheck) 1e+02))
      (bind _outactors (Collision|SphereOverlapActors (Transformation|GetActorLocation _asbp_enemy_base) (Variables|Default|GetRadiusCheck) (Utilities|Array|MakeArray "ObjectTypeQuery2") 0))
      (for _array_element _outactors
        (if (Actor|ActorHasTag _array_element "Cover")
          (if (< (Math|Vector|Distance(Vector) (Transformation|GetActorLocation _array_element) (Transformation|GetActorLocation _asbp_enemy_base)) (Variables|Default|GetMinDistance))
            (Variables|Default|SetMinDistance (Math|Vector|Distance(Vector) (Transformation|GetActorLocation _array_element) (Transformation|GetActorLocation _asbp_enemy_base)))
            (Variables|Default|SetTargetCover _array_element))))
      (Class|BTFunctionLibrary|SetBlackboardValueasObject (Variables|Default|GetBB_Cover) (Variables|Default|GetTargetCover))
      (AI|BehaviorTree|FinishExecute true))
    (:CastFailed
      (AI|BehaviorTree|FinishExecute false))))