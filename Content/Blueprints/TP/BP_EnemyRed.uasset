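; BP_EnemyRed is an enemy that loses health from hits or damage and can open a linked door when killed.
; OnHit and AnyDamage both subtract from Health and share one death check.
; At zero health it calls Death, notifies the player's BP_Weapon_Component of the kill, then opens LinkedDoor.
; The actor destroys itself here only if that door is valid, otherwise it prints a debug message.
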(event EventOnHit
  (params (Damage :type Float%20%28double-precision%29))
  (Variables|Default|Sethealth (- (Variables|Default|Gethealth) Damage))
  (Development|PrintString (Utilities|String|ToString(Float) 0.0))
  (if (<= (stale Game|Damage|EventAnyDamage _output_get) 0.0)
    (Utilities|FlowControl|Sequence
      (:then_0
        (Development|PrintString "preso")
        (CallFunction|Death))
      (:then_1
        (Default|OnEnemyKilled (Actor|GetComponentbyClass (Game|GetPlayerCharacter 0) "/Game/Blueprints/Components/BP_Weapon_Component.BP_Weapon_Component_C")))
      (:then_2
        (Utilities|IsValid (Variables|Default|GetLinkedDoor)
          (:Is%20Valid
            (Default|OpenDoor (Variables|Default|GetLinkedDoor))
            (Actor|DestroyActor))
          (:Is%20Not%20Valid
            (Development|PrintString "Non Trovato " true true "(R=1.000000,G=0.123850,B=0.944390,A=1.000000)")))))))

(event Game|Damage|EventAnyDamage
  (params (Damage :type Float%20%28single-precision%29) (DamageType :type Damage%20Type%20Object%20Reference) (InstigatedBy :type Controller%20Object%20Reference) (DamageCauser :type Actor%20Object%20Reference))
  (bind _output_get (Variables|Default|SetHealth (- (Variables|Default|GetHealth) Damage)))
  (if (<= _output_get 0.0)
    (Utilities|FlowControl|Sequence
      (:then_0
        (Development|PrintString "preso")
        (CallFunction|Death))
      (:then_1
        (Default|OnEnemyKilled (Actor|GetComponentbyClass (Game|GetPlayerCharacter 0) "/Game/Blueprints/Components/BP_Weapon_Component.BP_Weapon_Component_C")))
      (:then_2
        (Utilities|IsValid (Variables|Default|GetLinkedDoor)
          (:Is%20Valid
            (Default|OpenDoor (Variables|Default|GetLinkedDoor))
            (Actor|DestroyActor))
          (:Is%20Not%20Valid
            (Development|PrintString "Non Trovato " true true "(R=1.000000,G=0.123850,B=0.944390,A=1.000000)")))))))

(event EventBeginPlay
  (|CallParentFunction))

(fn ConstructionScript
  (|CallParentFunction))