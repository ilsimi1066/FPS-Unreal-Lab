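; Base enemy character with health, aim and crouch actions, and ranged attacks on the player.
; SphereTrace sweeps forward from the hand socket, spawns a projectile and damages the player if hit.
; OnHit and AnyDamage reduce a local Health variable, while BPHealthComponent's zero-health event also triggers Death.
; Death disables collision, stops the AI brain, notifies the player and fires a dispatcher; damage kills also notify the player's weapon component.
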(event Custom|OnDeath
  (CallFunction|Death))

(event EventOnHit
  (params (Damage :type Float%20%28double-precision%29))
  (Variables|Default|Sethealth (- (Variables|Default|Gethealth) Damage))
  (Development|PrintString (Utilities|String|ToString(Float) (- (Variables|Default|Gethealth) (stale Game|Damage|EventAnyDamage Damage))))
  (if (<= (Variables|Default|Gethealth) 0.0)
    (Utilities|FlowControl|Sequence
      (:then_0
        (Development|PrintString "preso")
        (CallFunction|Death))
      (:then_1
        (Default|OnEnemyKilled (Actor|GetComponentbyClass (Game|GetPlayerCharacter 0) "/Game/Blueprints/Components/BP_Weapon_Component.BP_Weapon_Component_C"))))))

(event EventBeginPlay
  (EventDispatchers|BindEventtoOnHealtZero (Variables|Default|GetBP_HealthComponent) (delegate Custom|OnDeath)))

(event Game|Damage|EventAnyDamage
  (params (Damage :type Float%20%28single-precision%29) (DamageType :type Damage%20Type%20Object%20Reference) (InstigatedBy :type Controller%20Object%20Reference) (DamageCauser :type Actor%20Object%20Reference))
  (Variables|Default|Sethealth (- (Variables|Default|Gethealth) Damage))
  (Development|PrintString (Utilities|String|ToString(Float) (- (Variables|Default|Gethealth) Damage)))
  (if (<= (Variables|Default|Gethealth) 0.0)
    (Utilities|FlowControl|Sequence
      (:then_0
        (Development|PrintString "preso")
        (CallFunction|Death))
      (:then_1
        (Default|OnEnemyKilled (Actor|GetComponentbyClass (Game|GetPlayerCharacter 0) "/Game/Blueprints/Components/BP_Weapon_Component.BP_Weapon_Component_C"))))))

(fn ConstructionScript)

(fn Aim
  (Default|CallOnAim))

(fn StopAim
  (Default|CallOnStopAim))

(fn GetFireStart
  (return (Transformation|GetSocketLocation (Variables|Character|GetMesh) "hand_rSocket") (Math|Vector|GetForwardVector (Variables|Collision|GetCapsuleComponent))))

(fn SphereTrace
  (bind (_position _dir) (CallFunction|GetFireStart))
  (bind _outhit (Collision|SphereTraceByChannel _position (+ _position (* _dir (.range (Variables|Default|GetWeaponInfo)))) 2e+01 "TraceTypeQuery2" false 0 "None"))
  (Game|SpawnActorfromClass "/Game/Blueprints/Gameplay/BP_projectile.BP_projectile_C" (Math|Transform|MakeTransform _position (Variables|/Script/Engine.SceneComponent|GetRelativeRotation (Variables|Collision|GetCapsuleComponent))) "Undefined" "MultiplyWithRoot" 0 0)
  (bind _asbp_first_person_character (Utilities|Casting|CastToBP_FirstPersonCharacter (.HitActor (Collision|BreakHitResult _outhit))))
  (Game|Damage|ApplyDamage _asbp_first_person_character (Variables|Default|Getdamage) 0 0))

(fn Death
  (Collision|SetCollisionEnabled (Variables|Collision|GetCapsuleComponent) "NoCollision")
  (Collision|SetCollisionEnabled (Variables|Character|GetMesh) "NoCollision")
  (bind _asbp_enemy_aicontroller (Utilities|Casting|CastToBP_EnemyAIController (AI|GetAIController self)))
  (Default|StopBrain _asbp_enemy_aicontroller)
  (bind _asbp_first_person_character (Utilities|Casting|CastToBP_FirstPersonCharacter (Game|GetPlayerCharacter 0)))
  (Default|OnEnemyKilledPlayer _asbp_first_person_character)
  (Default|CallOnDeathReached))

(fn CrouchMe
  (if (Class|Character|CanCrouch)
    (Character|Crouch)
    (Default|CallOnCrouch)))

(fn UncrouchMe
  (Character|UnCrouch)
  (Default|CallOnUncrouch))