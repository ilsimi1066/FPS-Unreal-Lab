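; Base enemy character, apparently for the tutorial, with hitscan shooting, aim and crouch actions broadcast through dispatchers.
; Shooting sphere-traces from the hand socket along capsule forward with persistent debug drawing, damaging only the first-person player.
; Death triggers from the health component or its own Health variable, stopping the AI brain and notifying the player.
; Lethal direct damage also destroys the actor and notifies the player's weapon component.
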(event Custom|OnDeath
  (CallFunction|Death))

(event EventBeginPlay
  (EventDispatchers|BindEventtoOnHealtZero (Variables|Default|GetBP_HealthComponent) (delegate Custom|OnDeath)))

(event Game|Damage|EventAnyDamage
  (params (Damage :type Float%20%28single-precision%29) (DamageType :type Damage%20Type%20Object%20Reference) (InstigatedBy :type Controller%20Object%20Reference) (DamageCauser :type Actor%20Object%20Reference))
  (Variables|Default|Sethealth (- (Variables|Default|Gethealth) Damage))
  (Development|PrintString (Utilities|String|ToString(Float) (- (Variables|Default|Gethealth) Damage)))
  (if (<= (Variables|Default|Gethealth) 0.0)
    (Variables|Default|SetHealth 0.0)
    (Utilities|FlowControl|Sequence
      (:then_0
        (Development|PrintString "preso")
        (CallFunction|Death)
        (Actor|DestroyActor))
      (:then_1
        (Default|OnEnemyKilled (Actor|GetComponentbyClass (Game|GetPlayerCharacter 0) "/Game/Blueprints/Components/BP_Weapon_Component.BP_Weapon_Component_C"))))))

(fn ConstructionScript)

(fn Aim
  (Default|CallOnAim))

(fn StopAim
  (Default|CallOnStopAim))

(fn GetFireStart
  (return (Transformation|GetSocketLocation (Variables|Character|GetMesh) "hand_rSocket") (Math|Vector|GetForwardVector (Variables|Collision|GetCapsuleComponent))))

(fn SphereTrace
  (bind (_position _dir) (CallFunction|GetFireStart))
  (bind _weaponinfo (Variables|Default|GetWeaponInfo))
  (bind _outhit (Collision|SphereTraceByChannel _position (+ _position (* _dir (.range _weaponinfo))) 2e+01 "TraceTypeQuery2" false 0 "Persistent"))
  (bind _asbp_first_person_character (Utilities|Casting|CastToBP_FirstPersonCharacter (.HitActor (Collision|BreakHitResult _outhit))))
  (Game|Damage|ApplyDamage _asbp_first_person_character (.damage _weaponinfo) 0 0 "/Script/Engine.DamageType"))

(fn Death
  (bind _asbp_enemy_aicontroller (Utilities|Casting|CastToBP_EnemyAIController (AI|GetAIController self)))
  (Default|StopBrain _asbp_enemy_aicontroller)
  (bind _asbp_first_person_character (Utilities|Casting|CastToBP_FirstPersonCharacter (Game|GetPlayerCharacter 0)))
  (Utilities|FlowControl|Sequence
    (:then_0
      (Utilities|FlowControl|DoOnce false
        (:Completed
          (Default|OnEnemyKilledPlayer _asbp_first_person_character))))
    (:then_1
      (Default|CallOnDeathReached))))

(fn CrouchMe
  (if (Class|Character|CanCrouch)
    (Character|Crouch)
    (Default|CallOnCrouch)))

(fn UncrouchMe
  (Character|UnCrouch)
  (Default|CallOnUncrouch))