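; BP_enemyNucleo is a "nucleo" enemy that takes damage and dies.
; AnyDamage subtracts from its own Health0 and, at zero or below, frees its spawn point, calls Death and notifies the player's weapon component of the kill.
; The health component's zero-health event also calls Death, but damage is never forwarded to that component.
; Debug prints trace damage and death.
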(event Custom|OnDeath
  (CallFunction|Death))

(event EventBeginPlay
  (EventDispatchers|BindEventtoOnHealtZero (Variables|Default|GetBP_HealthComponent1) (delegate Custom|OnDeath)))

(event Game|Damage|EventAnyDamage
  (params (Damage :type Float%20%28single-precision%29) (DamageType :type Damage%20Type%20Object%20Reference) (InstigatedBy :type Controller%20Object%20Reference) (DamageCauser :type Actor%20Object%20Reference))
  (bind _myspawnpoint (Variables|Default|GetMySpawnPoint))
  (Variables|Default|SetHealth_0 (- (Variables|Default|GetHealth_0) Damage))
  (Development|PrintString (Utilities|String|ToString(Float) (- (Variables|Default|GetHealth_0) Damage)))
  (if (<= (Variables|Default|GetHealth_0) 0.0)
    (Utilities|FlowControl|Sequence
      (:then_0
        (Utilities|IsValid _myspawnpoint
          (:Is%20Valid
            (Variables|/Game/Blueprints/BP_Enemy_SpawnPoint.BP_Enemy_SpawnPoint_C|SetIsOccupied _myspawnpoint false))
          (:Is%20Not%20Valid
            _))
        (Development|PrintString "preso")
        (CallFunction|Death))
      (:then_1
        (Default|OnEnemyKilled (Actor|GetComponentbyClass (Game|GetPlayerCharacter 0) "/Game/Blueprints/Components/BP_Weapon_Component.BP_Weapon_Component_C"))))))

(fn ConstructionScript)