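; BP_EnemyAIController is an AI controller for enemies that runs a behavior tree on BeginPlay.
; When AI perception updates, it finds the first-person player character and sets the seePlayer blackboard key if the first sense's stimulus is successfully sensed.
; The key is only ever set to true here, never cleared.
; StopBrain halts the behavior tree logic and stops movement.
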(event OnPerceptionUpdated(AIPerception)
  (params (UpdatedActors :type Array%20of%20Actor%20Object%20References))
  (for _array_element UpdatedActors
    (bind _asbp_first_person_character (Utilities|Casting|CastToBP_FirstPersonCharacter _array_element))
    (bind _info (Class|AIPerceptionComponent|GetActorsPerception (Variables|Default|GetAIPerception) _asbp_first_person_character))
    (for (_array_element_2 _array_index) (.LastSensedStimuli (Utilities|Struct|BreakActorPerceptionBlueprintInfo _info))
      (if (.bSuccessfullySensed (Utilities|Struct|BreakAIStimulus _array_element_2))
        (switch int _array_index
          (:0
            (AI|Components|Blackboard|SetValueasBool (AI|GetBlackboard 0) (Utilities|Name|MakeLiteralName "seePlayer") true)))))))

(event EventBeginPlay
  (AI|RunBehaviorTree (Variables|Default|GetMyBehaviourTree)))

(fn ConstructionScript)

(fn StopBrain
  (AI|Logic|StopLogic (Variables|Default|GetBrainComponent) "")
  (AI|Navigation|StopMovement))