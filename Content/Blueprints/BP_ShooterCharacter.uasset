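; BP_ShooterCharacter is a shooter character Blueprint that exposes its mesh and the start and end points of a line of fire.
; RetrieveCharacterMesh returns the Mesh component.
; GetFireStart returns the capsule's world location, and GetFireEnd projects from there along the capsule's forward vector by the given Range, so aim follows the capsule's facing.
; The event graph and construction script contain no logic.
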(event EventBeginPlay)

(event Collision|EventActorBeginOverlap
  (params (OtherActor :type Actor%20Object%20Reference)))

(event EventTick
  (params (DeltaSeconds :type Float%20%28single-precision%29)))

(fn ConstructionScript)

(fn RetrieveCharacterMesh
  (return (Variables|Character|GetMesh)))

(fn GetFireStart
  (return (Transformation|GetWorldLocation (Variables|Collision|GetCapsuleComponent))))

(fn GetFireEnd
  (params (Range :type Float%20%28double-precision%29))
  (bind _capsulecomponent (Variables|Collision|GetCapsuleComponent))
  (return (+ (Transformation|GetWorldLocation _capsulecomponent) (* Range (Math|Vector|GetForwardVector _capsulecomponent)))))