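; BP_Target is a damageable target, treated as an enemy, that tracks its Health and is destroyed when killed.
; AnyDamage subtracts damage from Health and, at zero or below, fires OnEnemyKilled, whose event destroys the actor.
; It then notifies player 0's BP_FirstPersonCharacter and BP_Weapon_Component of the kill, regardless of who dealt the damage.
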(event Custom|onEnemyKilled
  (Actor|DestroyActor))

(event Game|Damage|EventAnyDamage
  (params (Damage :type Float%20%28single-precision%29) (DamageType :type Damage%20Type%20Object%20Reference) (InstigatedBy :type Controller%20Object%20Reference) (DamageCauser :type Actor%20Object%20Reference))
  (Variables|Default|Sethealth (- (Variables|Default|Gethealth) Damage))
  (if (<= (Variables|Default|Gethealth) 0.0)
    (Utilities|FlowControl|Sequence
      (:then_0
        (CallFunction|OnEnemyKilled)
        (bind _asbp_first_person_character (Utilities|Casting|CastToBP_FirstPersonCharacter (Game|GetPlayerCharacter 0)))
        (Default|OnEnemyKilledPlayer _asbp_first_person_character))
      (:then_1
        (Default|OnEnemyKilled (Actor|GetComponentbyClass (Game|GetPlayerCharacter 0) "/Game/Blueprints/Components/BP_Weapon_Component.BP_Weapon_Component_C"))))))

(fn ConstructionScript)